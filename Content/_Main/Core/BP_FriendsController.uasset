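; BP_FriendsController sets up the friends list, its global MVVM viewmodel and the friend characters, and simulates friends coming online and offline.
; On BeginPlay it loads the initial list into FriendsListControllerComponent's database, which FriendCharactersManagerComponent uses to spawn characters.
; Component change events push online, offline and last-connected users into VM_FriendsList, registered in the global viewmodel collection.
; A self-calling delayed event randomly reconnects or disconnects a player at a set interval.
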(event `self.ReceiveBeginPlay`
  (`self.AppendInitialFriendsListToDatabase`)
  (`self.InitGlobalFriendsListViewmodel`)
  (add `FriendsListControllerComponent.OnlineUsersChanged` (`self.FriendsListControllerComponent`) (`|CreateDelegate` :!event `OnOnlineUsersChanged`))
  (add `FriendsListControllerComponent.OfflineUsersChanged` (`self.FriendsListControllerComponent`) (`|CreateDelegate` :!event `OnOfflineUsersChanged`))
  (add `FriendsListControllerComponent.LastConnectedUserChanged` (`self.FriendsListControllerComponent`) (`|CreateDelegate` :!event `OnLastConnectedUserChanged`))
  (`FriendCharactersManagerComponent.SpawnAndSetupFriendCharacters` (`self.FriendCharactersManagerComponent`) (`FriendsListControllerComponent.Database` (`self.FriendsListControllerComponent`)))
  (`self.SimulateConstantConnectionStateChange`))

(event `SimulateConstantConnectionStateChange`
  (`KismetSystemLibrary.Delay` (`self.ConnectionChangeIntervalSeconds`))
  (`FriendsListControllerComponent.ReconnectOrDisconnectRandomPlayer` (`self.FriendsListControllerComponent`))
  (`self.SimulateConstantConnectionStateChange`))

(fn `AppendInitialFriendsListToDatabase`
  (`FriendsListControllerComponent.AppendToDatabase` (`self.FriendsListControllerComponent`) (`FriendsListDataAsset.Content` (`self.InitialFriendsList`))))

(fn `InitGlobalFriendsListViewmodel`
  (bind _friendslistcontrollercomponent (`self.FriendsListControllerComponent`))
  (`self.VM_FriendsList`
    (:`then`
      _)
    (:`else`
      (bind _returnvalue (`|GenericCreateObject` "/Game/_Main/Core/VM_FriendsList.VM_FriendsList_C" (`FriendsListControllerComponent.OnlineUsersCached` _friendslistcontrollercomponent) (`FriendsListControllerComponent.OfflineUsersCached` _friendslistcontrollercomponent)))
      (set `self.VM_FriendsList` _returnvalue)))
  (`MVVMViewModelCollectionObject.AddViewModelInstance` (`MVVMGameSubsystem.GetViewModelCollection` (subsystem `MVVMGameSubsystem`)) (make `MVVMViewModelContext` "/Game/_Main/Core/VM_FriendsList.VM_FriendsList_C" "VM_FriendsList") (`self.VM_FriendsList`)))

(fn `OnLastConnectedUserChanged`
  (params (Value :type "DefaultUserDataWrapper Object Reference"))
  (set `/Game/_Main/Core/VM_FriendsList.LastConnectedUser` Value (`self.VM_FriendsList`)))

(fn `OnOfflineUsersChanged`
  (set `/Game/_Main/Core/VM_FriendsList.OfflineUsers` (`FriendsListControllerComponent.OfflineUsersCached` (`self.FriendsListControllerComponent`)) (`self.VM_FriendsList`)))

(fn `OnOnlineUsersChanged`
  (set `/Game/_Main/Core/VM_FriendsList.OnlineUsers` (`FriendsListControllerComponent.OnlineUsersCached` (`self.FriendsListControllerComponent`)) (`self.VM_FriendsList`)))

(fn `UserConstructionScript`)