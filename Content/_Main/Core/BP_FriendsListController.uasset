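; Controller Blueprint that owns the friends list data and exposes it to UI through a global MVVM viewmodel.
; Its construction script appends an initial list to the FriendsListControllerComponent database, creates VM_FriendsList if needed and registers it in the MVVM global viewmodel collection.
; It also binds to the component's database state changes, with a handler that refreshes the viewmodel's content from the database as UObjects.
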(fn `AppendInitialFriendsListToDatabase`
  (`KismetArrayLibrary.Array_Append` (`FriendsListControllerComponent.Database` (`self.FriendsListControllerComponent`)) (`FriendsListDataAsset.Content` (`self.InitialFriendsList`))))

(fn `InitGlobalFriendsListViewmodel`
  (`self.VM_FriendsList`
    (:`then`
      _)
    (:`else`
      (`|GenericCreateObject` "/Game/_Main/Core/VM_FriendsList.VM_FriendsList_C" (`FriendsListControllerComponent.GetDatabaseAsUObjects` (`self.FriendsListControllerComponent`)))))
  (`MVVMViewModelCollectionObject.AddViewModelInstance` (`MVVMGameSubsystem.GetViewModelCollection` (subsystem `MVVMGameSubsystem`)) (make `MVVMViewModelContext` "/Game/_Main/Core/VM_FriendsList.VM_FriendsList_C" "VM_FriendsList") (`self.VM_FriendsList`)))

(fn `OnDatabaseStateChanged`
  (set `/Game/_Main/Core/VM_FriendsList.Content` (`FriendsListControllerComponent.GetDatabaseAsUObjects` (`self.FriendsListControllerComponent`)) (`self.VM_FriendsList`)))

(fn `UserConstructionScript`
  (`self.AppendInitialFriendsListToDatabase`)
  (`self.InitGlobalFriendsListViewmodel`)
  (add `FriendsListControllerComponent.DatabaseStateChanged` (`self.FriendsListControllerComponent`) (`|CreateDelegate` :!event `OnDatabaseStateChanged`)))