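; BP_FriendBase is a base Blueprint for a friend representation that shows a user's status through a WBP_FriendsListItem status widget.
; BeginPlay caches the list item from the StatusWidget component.
; Setup stores the user data, applies its source data immediately and binds to source-data changes.
; Each update derives IsOnline from the connection state, calls CallIsOnlineChanged with it and refreshes the widget.
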(event `self.ReceiveBeginPlay`
  (bind _aswbp_friends_list_item (cast `/Game/_Main/UI/WBP_FriendsListItem` (`WidgetComponent.GetUserWidgetObject` (`self.StatusWidget`))))
  (set `self.WBP_FriendsListItem` _aswbp_friends_list_item))

(event `self.Setup`
  (params (UserData :type "DefaultUserDataWrapper Object Reference"))
  (bind _output_get (set `self.UserData` UserData))
  (`self.OnSourceDataChanged` (`DefaultUserDataWrapper.SourceData` _output_get))
  (add `DefaultUserDataWrapper.SourceDataChanged` (`self.UserData`) (`|CreateDelegate` :!event `OnSourceDataChanged`)))

(fn `OnSourceDataChanged`
  (params (NewValue :type "DefaultUserData Structure"))
  (bind _output_get (set `self.IsOnline` (`|EnumEquality` NewValue_ConnectionState "Online")))
  (`self.IsOnlineChanged` _output_get)
  (`/Game/_Main/UI/WBP_FriendsListItem.UpdateWidget` (`self.WBP_FriendsListItem`) (`self.UserData`)))

(fn `UserConstructionScript`)